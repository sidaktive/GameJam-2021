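; Player character Blueprint that picks up and throws balls, with state changes routed through Server events.
; Server events track the overlapped ball; E picks it up, pausing its movement and physics, attaching it to a hand socket and recording the holder.
; Left-click press only debug-draws a suggested trajectory toward the cursor.
; Release detaches the ball, reactivates it and applies camera-forward plus fixed upward-biased forces.
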(event `Server_ClearOverlappedBall`
  (set `self.OverlappedBall` null))

(event `Server_SetOverlappedBall`
  (params (OverlappedBall :type "/Game/StarterProject/Blueprints/BP_Handheld_Ball Object Reference"))
  (set `self.OverlappedBall` OverlappedBall)
  (`KismetSystemLibrary.PrintString` "Overlapped ball!"))

(event `Key|E`
  (params (Key :type "Key Structure"))
  (:`Pressed`
    (`self.HeldBall`
      (:`then`)
      (:`else`
        (bind _overlappedball (`self.OverlappedBall`)
          (:`then`
            (`self.Server_PickUpBall` _overlappedball))
          (:`else`
            (`KismetSystemLibrary.PrintString` "no overlapped ball")))))))

(event `Server_PickUpBall`
  (params (Ball :type "/Game/StarterProject/Blueprints/BP_Handheld_Ball Object Reference"))
  (bind _output_get (set `self.HeldBall` Ball))
  (set `/Game/StarterProject/Blueprints/BP_Handheld_Ball.isHeld` true _output_get)
  (`ActorComponent.Deactivate` (`/Game/StarterProject/Blueprints/BP_Handheld_Ball.ProjectileMovement` _output_get))
  (`PrimitiveComponent.SetSimulatePhysics` (`/Game/StarterProject/Blueprints/BP_Handheld_Ball.StaticMesh` _output_get) false)
  (`self.SetActorRelativeScale3D` _output_get (1.0 1.0 1.0))
  (`self.K2_AttachToComponent` _output_get (`self.Mesh`) "middle_01_r" "SnapToTarget" "SnapToTarget" "KeepWorld" true)
  (set `/Game/StarterProject/Blueprints/BP_Handheld_Ball.lastHeldBy` self _output_get))

(event `Key|LeftMouseButton`
  (params (Key :type "Key Structure"))
  (:`Pressed`
    (bind _heldball (`self.HeldBall`)
      (:`then`
        (`GameplayStatics.BlueprintSuggestProjectileVelocity` (`self.K2_GetActorLocation` _heldball) (`PlayerController.DeprojectMousePositionToWorld` (`GameplayStatics.GetPlayerController` 0)) 30000.0 0.0 "TraceFullPath" 0.0 false true))
      (:`else`))))

(event `Key|LeftMouseButton`
  (params (Key :type "Key Structure"))
  (:`Released`
    (`self.HeldBall`
      (:`then`
        (`self.Server_ThrowBall`))
      (:`else`))))

(event `Server_ThrowBall`
  (bind _staticmesh (`/Game/StarterProject/Blueprints/BP_Handheld_Ball.StaticMesh` (`self.HeldBall`)))
  (bind _heldball (`self.HeldBall`)
    (:`then`
      (`SceneComponent.K2_DetachFromComponent` (`Actor.RootComponent` _heldball) "KeepWorld" "KeepWorld" "KeepWorld" true)
      (`ActorComponent.Activate` (`/Game/StarterProject/Blueprints/BP_Handheld_Ball.ProjectileMovement` _heldball) false)
      (`PrimitiveComponent.SetSimulatePhysics` (`/Game/StarterProject/Blueprints/BP_Handheld_Ball.StaticMesh` _heldball) true)
      (`PrimitiveComponent.AddForce` _staticmesh (* (`SceneComponent.GetForwardVector` (`self.FollowCamera`)) 200000.0) "None" true)
      (`PrimitiveComponent.AddForce` _staticmesh (500.0 500.0 18000.0) "None" true)
      (set `/Game/StarterProject/Blueprints/BP_Handheld_Ball.isHeld` false _heldball)
      (set `self.HeldBall` null))
    (:`else`)))

(fn `OnRep_OverlappedBall`)

(fn `UserConstructionScript`)