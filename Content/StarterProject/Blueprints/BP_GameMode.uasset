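; Game mode that handles player respawning and balanced red/blue team assignment.
; On authority, respawn requests spawn a PlayerCharacter_BP at the supplied transform and possess it after a short delay.
; Team requests set the PlayerState team to the smaller side, with ties going blue, and increment its count.
; It also creates a HUD widget, binds a death handler calling DestroyActor, and caches PlayerStarts during construction.
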(event `self.ReceiveBeginPlay`
  (bind _hudwidget (`self.HUDWidget`))
  (add `self.OnPlayerDied` (delegate `PlayerDead`))
  (`/Engine/EditorBlueprintResources/StandardMacros.IsValid` _hudwidget
    (:`Is Valid`
      (`UserWidget.AddToViewport` _hudwidget 0))
    (:`Is Not Valid`
      (bind _returnvalue (`|CreateWidget` "/Game/StarterProject/Widgets/W_PlayerHUD.W_PlayerHUD_C"))
      (set `self.HUDWidget` _returnvalue))))

(event `PlayerDead` :!signature `self.OnPlayerDied`
  (params (Character :type "Character Object Reference"))
  (`self.K2_DestroyActor`))

(event `RespawnRequested`
  (params (PlayerController :type "PlayerController Object Reference") (SpawnTransform :type "Transform Structure"))
  (`/Engine/EditorBlueprintResources/StandardMacros.IsValid` PlayerController
    (:`Is Valid`
      (`/Engine/EditorBlueprintResources/ActorMacros.Switch Has Authority`
        (:`Authority`
          (cast `/Game/StarterProject/Blueprints/BP_PlayerState` (`Controller.PlayerState` PlayerController))
          (bind _returnvalue (`|SpawnActorFromClass` "/Game/StarterProject/Characters/PlayerCharacter_BP.PlayerCharacter_BP_C" SpawnTransform "Undefined" "OverrideRootScale" null null))
          (`KismetSystemLibrary.Delay` 0.2)
          (`Controller.Possess` PlayerController _returnvalue))))))

(event `TeamAllocationRequested`
  (params (`Player Controller` :type "PlayerController Object Reference"))
  (bind _redteamsize (`self.RedTeamSize`))
  (bind _blueteamsize (`self.BlueTeamSize`))
  (`/Engine/EditorBlueprintResources/StandardMacros.IsValid` `Player Controller`
    (:`Is Valid`
      (`/Engine/EditorBlueprintResources/ActorMacros.Switch Has Authority`
        (:`Authority`
          (bind _asbp_player_controller (cast `/Game/StarterProject/Blueprints/BP_PlayerController` `Player Controller`))
          (bind _asbp_player_state (cast `/Game/StarterProject/Blueprints/BP_PlayerState` (`Controller.PlayerState` _asbp_player_controller)))
          (`/Engine/EditorBlueprintResources/StandardMacros.CompareInt` _redteamsize _blueteamsize
            (:`>`
              (set `/Game/StarterProject/Blueprints/BP_PlayerState.PlayerTeam` "NewEnumerator1" _asbp_player_state :!label _label)
              (bind _result (`/Engine/EditorBlueprintResources/StandardMacros.IncrementInt` _blueteamsize)
                (:`  `
                  (set `self.BlueTeamSize` _result))))
            (:`==`
              (goto _label))
            (:`<`
              (set `/Game/StarterProject/Blueprints/BP_PlayerState.PlayerTeam` "NewEnumerator0" _asbp_player_state)
              (bind _result_2 (`/Engine/EditorBlueprintResources/StandardMacros.IncrementInt` _redteamsize)
                (:`  `
                  (set `self.RedTeamSize` _result_2))))))))))

(fn `UserConstructionScript`
  (bind _outactors (`GameplayStatics.GetAllActorsOfClass` "/Script/Engine.PlayerStart"))
  (set `self.PlayerStarts` _outactors))