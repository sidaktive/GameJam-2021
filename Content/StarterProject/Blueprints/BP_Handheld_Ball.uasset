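; BP_Handheld_Ball is a ball actor that player characters can overlap and be hit by.
; On the server, actor overlaps set or clear the overlapped ball on PlayerCharacter_BP.
; When unheld, its collision sphere treats overlap with a player other than the valid last holder as a hit, without an authority check.
; The hit calls OnPlayerHitByBall, which only prints a respawn message.
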(event `self.ReceiveActorBeginOverlap`
  (params (OtherActor :type "Actor Object Reference"))
  (`/Engine/EditorBlueprintResources/ActorMacros.Switch Has Authority`
    (:`Authority`
      (bind _asplayer_character_bp (cast `/Game/StarterProject/Characters/PlayerCharacter_BP` OtherActor))
      (`/Game/StarterProject/Characters/PlayerCharacter_BP.Server_SetOverlappedBall` _asplayer_character_bp self))))

(event `self.ReceiveActorEndOverlap`
  (params (OtherActor :type "Actor Object Reference"))
  (`/Engine/EditorBlueprintResources/ActorMacros.Switch Has Authority`
    (:`Authority`
      (bind _asplayer_character_bp (cast `/Game/StarterProject/Characters/PlayerCharacter_BP` OtherActor))
      (`/Game/StarterProject/Characters/PlayerCharacter_BP.Server_ClearOverlappedBall` _asplayer_character_bp))))

(event `self.Coll_Sphere.OnComponentBeginOverlap`
  (params (OverlappedComponent :type "PrimitiveComponent Object Reference") (OtherActor :type "Actor Object Reference") (OtherComp :type "PrimitiveComponent Object Reference") (OtherBodyIndex :type Integer) (bFromSweep :type Boolean) (SweepResult :type "HitResult Structure (by ref)"))
  (bind _lastheldby (`self.lastHeldBy`))
  (if (not (`self.isHeld`))
    (`/Engine/EditorBlueprintResources/StandardMacros.IsValid` _lastheldby
      (:`Is Valid`
        (if (not (== _lastheldby OtherActor))
          (`KismetSystemLibrary.PrintString` (`KismetStringLibrary.Concat_StrStr` "Collided with:" (`KismetSystemLibrary.GetDisplayName` OtherActor) "| Last Held By:" (`KismetSystemLibrary.GetDisplayName` _lastheldby)))
          (bind _asplayer_character_bp (cast `/Game/StarterProject/Characters/PlayerCharacter_BP` OtherActor))
          (`self.On Player Hit By Ball` _asplayer_character_bp))))))

(event `On Player Hit By Ball`
  (params (`Player Character` :type "/Game/StarterProject/Characters/PlayerCharacter_BP Object Reference"))
  (`KismetSystemLibrary.PrintString` "Respawning Character"))

(fn `UserConstructionScript`)